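; Player character with switchable red, green and blue colour modes, plus wall climbing and egg spawning.
; Keys 1-3 set HUD mode flags and recolour a dynamic body material, starting blue.
; Hits while off the ground briefly raise the jump limit for climbing, despite its "green" label working in any mode.
; E spawns the Spawnable by the mesh when InternalIsBlue is set, a flag that never clears.
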(event Custom|Red
  (bind _ashud_first_blood (Utilities|Casting|CastToHUD_FirstBlood (HUD|GetHUD (Game|GetPlayerController 0))))
  (Variables|/Game/Tut_FirstBlood/Blueprints/HUD_FirstBlood.HUD_FirstBlood_C|SetGreenMode _ashud_first_blood false)
  (Variables|/Game/Tut_FirstBlood/Blueprints/HUD_FirstBlood.HUD_FirstBlood_C|SetBlueMode _ashud_first_blood false)
  (Variables|/Game/Tut_FirstBlood/Blueprints/HUD_FirstBlood.HUD_FirstBlood_C|SetRedMode _ashud_first_blood true))

(event Custom|Green
  (bind _ashud_first_blood (Utilities|Casting|CastToHUD_FirstBlood (HUD|GetHUD (Game|GetPlayerController 0))))
  (Variables|/Game/Tut_FirstBlood/Blueprints/HUD_FirstBlood.HUD_FirstBlood_C|SetBlueMode _ashud_first_blood false)
  (Variables|/Game/Tut_FirstBlood/Blueprints/HUD_FirstBlood.HUD_FirstBlood_C|SetRedMode _ashud_first_blood false)
  (bind _output_get (Variables|/Game/Tut_FirstBlood/Blueprints/HUD_FirstBlood.HUD_FirstBlood_C|SetGreenMode _ashud_first_blood true))
  (Variables|Default|SetinternalIsGreen _output_get))

(event Custom|Blue
  (bind _ashud_first_blood (Utilities|Casting|CastToHUD_FirstBlood (HUD|GetHUD (Game|GetPlayerController 0))))
  (Variables|/Game/Tut_FirstBlood/Blueprints/HUD_FirstBlood.HUD_FirstBlood_C|SetRedMode _ashud_first_blood false)
  (Variables|/Game/Tut_FirstBlood/Blueprints/HUD_FirstBlood.HUD_FirstBlood_C|SetGreenMode _ashud_first_blood false)
  (bind _output_get (Variables|/Game/Tut_FirstBlood/Blueprints/HUD_FirstBlood.HUD_FirstBlood_C|SetBlueMode _ashud_first_blood true))
  (Variables|Default|SetinternalIsBlue _output_get))

(event EventBeginPlay
  (CallFunction|Blue)
  (Rendering|Material|SetVectorParameterValue (Variables|Default|GetcharacterMat) "BodyColor" "(R=0.013376,G=0.000000,B=1.000000,A=1.000000)" :!class /Script/Engine.MaterialInstanceDynamic))

(event Collision|EventActorBeginOverlap
  (params (OtherActor :type Actor%20Object%20Reference)))

(event EventTick
  (params (DeltaSeconds :type Float%20%28single-precision%29))
  ;[1 1 1] Green climbing power
  (if (Variables|Default|GetisOnWall)
    (Variables|Default|SetJumpMaxCount 500)
    (Variables|Default|SetisOnWall false)
    (else
      (Variables|Default|SetJumpMaxCount 1))))

(event Collision|EventHit
  (params (MyComp :type Primitive%20Component%20Object%20Reference) (Other :type Actor%20Object%20Reference) (OtherComp :type Primitive%20Component%20Object%20Reference) (bSelfMoved :type Boolean) (HitLocation :type Vector :default "0, 0, 0") (HitNormal :type Vector :default "0, 0, 0") (NormalImpulse :type Vector :default "0, 0, 0") (Hit :type Hit%20Result%20Structure%20%28by%20ref%29))
  ;[1 1 1] Green climbing power
  (Variables|Default|SetisOnWall (not (AI|Components|NavMovement|IsMovingonGround (Variables|Character|GetCharacterMovement)))))

(event Input|KeyboardEvents|1
  (params (Key :type Key%20Structure :default "None"))
  (:Pressed
    (CallFunction|Red)
    (Rendering|Material|SetVectorParameterValue (Variables|Default|GetcharacterMat) "BodyColor" "(R=1.000000,G=0.000000,B=0.000000,A=1.000000)" :!class /Script/Engine.MaterialInstanceDynamic)))

(event Input|KeyboardEvents|2
  (params (Key :type Key%20Structure :default "None"))
  (:Pressed
    (CallFunction|Green)
    (Rendering|Material|SetVectorParameterValue (Variables|Default|GetcharacterMat) "BodyColor" "(R=0.013145,G=1.000000,B=0.000000,A=1.000000)" :!class /Script/Engine.MaterialInstanceDynamic)))

(event Input|KeyboardEvents|3
  (params (Key :type Key%20Structure :default "None"))
  (:Pressed
    (CallFunction|Blue)
    (Rendering|Material|SetVectorParameterValue (Variables|Default|GetcharacterMat) "BodyColor" "(R=0.013376,G=0.000000,B=1.000000,A=1.000000)" :!class /Script/Engine.MaterialInstanceDynamic)))

(event Input|KeyboardEvents|E
  (params (Key :type Key%20Structure :default "None"))
  (bind _mesh (Variables|Character|GetMesh))
  ;[1 1 1] Blue power spawn an egg
  (:Pressed
    (if (Variables|Default|GetinternalIsBlue)
      (Game|SpawnActorfromClass "/Game/Tut_FirstBlood/Blueprints/Spawnable.Spawnable_C" (Math|Conversions|ToTransform(Vector) (+ (* (Math|Vector|GetForwardVector (Transformation|GetWorldRotation _mesh)) 1e+01) (Transformation|GetWorldLocation _mesh))) "Undefined" 0 0))))

(fn ConstructionScript
  (bind _returnvalue (Rendering|Material|CreateDynamicMaterialInstance (Variables|Character|GetMesh) 0 0 "None" :!class /Script/Engine.PrimitiveComponent))
  (Variables|Default|SetcharacterMat _returnvalue))