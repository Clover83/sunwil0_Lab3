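; Coin is a pickup actor that spins and adds to the player's score when hit by the player character.
; Tick rotates it around yaw at YawPerSecond, scaled by delta time.
; A hit on its Cylinder component from MyCharacter increments Score directly on HUD_FirstBlood, then destroys the coin.
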(event OnComponentHit(Cylinder)
  (params (HitComponent :type Primitive%20Component%20Object%20Reference) (OtherActor :type Actor%20Object%20Reference) (OtherComp :type Primitive%20Component%20Object%20Reference) (NormalImpulse :type Vector :default "0, 0, 0") (Hit :type Hit%20Result%20Structure%20%28by%20ref%29))
  (Utilities|Casting|CastToMyCharacter OtherActor)
  (bind _ashud_first_blood (Utilities|Casting|CastToHUD_FirstBlood (HUD|GetHUD (Game|GetPlayerController 0))))
  (Variables|/Game/Tut_FirstBlood/Blueprints/HUD_FirstBlood.HUD_FirstBlood_C|SetScore _ashud_first_blood (+ (Variables|/Game/Tut_FirstBlood/Blueprints/HUD_FirstBlood.HUD_FirstBlood_C|GetScore _ashud_first_blood) 1))
  (Actor|DestroyActor))

(event EventBeginPlay)

(event Collision|EventActorBeginOverlap
  (params (OtherActor :type Actor%20Object%20Reference)))

(event EventTick
  (params (DeltaSeconds :type Float%20%28single-precision%29))
  (Transformation|AddActorLocalRotation (Math|Rotator|MakeRotator 0.0 0.0 (* (Variables|Default|GetyawPerSecond) DeltaSeconds)) false false))

(fn ConstructionScript)