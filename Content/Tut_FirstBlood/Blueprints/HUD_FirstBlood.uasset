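; HUD Blueprint for the FirstBlood tutorial that draws a color-coded fullscreen overlay and the score counter.
; Each DrawHUD call stretches the blue, red or green material across the screen according to the mode booleans, checked in that order, and sets BlueMode if none is active.
; It then draws a coin material and the Score value near the top-right, positioned relative to screen width.
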(event EventBeginPlay)

(event Collision|EventActorBeginOverlap
  (params (OtherActor :type Actor%20Object%20Reference)))

(event EventTick
  (params (DeltaSeconds :type Float%20%28single-precision%29)))

(event EventDrawHUD
  (params (SizeX :type Integer) (SizeY :type Integer))
  (Variables|Default|SetsizeX SizeX)
  (Variables|Default|SetsizeY SizeY)
  (Utilities|FlowControl|Sequence
    (:then_0
      (if (Variables|Default|GetBlueMode)
        (Class|HUD|DrawMaterialSimple "/Game/Tut_FirstBlood/Textures/Mat_HUDB.Mat_HUDB" 0.0 0.0 (Math|Conversions|ToFloat(Integer) (Variables|Default|GetsizeX)) (Math|Conversions|ToFloat(Integer) (Variables|Default|GetsizeY)) 1.0 false)
        (elif (Variables|Default|GetRedMode)
          (Class|HUD|DrawMaterialSimple "/Game/Tut_FirstBlood/Textures/Mat_HUDR.Mat_HUDR" 0.0 0.0 (Math|Conversions|ToFloat(Integer) (Variables|Default|GetsizeX)) (Math|Conversions|ToFloat(Integer) (Variables|Default|GetsizeY)) 1.0 false)
          (elif (Variables|Default|GetGreenMode)
            (Class|HUD|DrawMaterialSimple "/Game/Tut_FirstBlood/Textures/Mat_HUDG.Mat_HUDG" 0.0 0.0 (Math|Conversions|ToFloat(Integer) (Variables|Default|GetsizeX)) (Math|Conversions|ToFloat(Integer) (Variables|Default|GetsizeY)) 1.0 false)
            (else
              (Variables|Default|SetBlueMode true))))))
    (:then_1
      (Class|HUD|DrawMaterialSimple "/Game/Tut_FirstBlood/Textures/MAT_Coin.MAT_Coin" (- (Math|Conversions|ToFloat(Integer) (Variables|Default|GetsizeX)) 2.5e+02) 1e+02 1e+02 1e+02 1.0 false)
      (HUD|DrawText "x" "(R=1.000000,G=1.000000,B=1.000000,A=1.000000)" (- (Math|Conversions|ToFloat(Integer) (Variables|Default|GetsizeX)) 1.5e+02) 1.2e+02 "/Engine/EngineFonts/RobotoDistanceField.RobotoDistanceField" 2.5 false)
      (HUD|DrawText (Utilities|String|ToString(Integer) (Variables|Default|GetScore)) "(R=1.000000,G=1.000000,B=1.000000,A=1.000000)" (- (Math|Conversions|ToFloat(Integer) (Variables|Default|GetsizeX)) 1.1e+02) 1.2e+02 "/Engine/EngineFonts/RobotoDistanceField.RobotoDistanceField" 2.5 false))))

(fn ConstructionScript)