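; Player character for the FirstBlood tutorial that switches between red, green and blue modes with the 1, 2 and 3 keys.
; Each mode event sets exclusive RedMode, GreenMode and BlueMode flags on HUD_FirstBlood.
; The construction script creates a dynamic material instance on the mesh, whose BodyColor parameter is then set to match the chosen mode.
; Play begins in blue mode.
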(event Custom|Red
  (bind _ashud_first_blood (Utilities|Casting|CastToHUD_FirstBlood (HUD|GetHUD (Game|GetPlayerController 0))))
  (Variables|/Game/Tut_FirstBlood/Blueprints/HUD_FirstBlood.HUD_FirstBlood_C|SetGreenMode _ashud_first_blood false)
  (Variables|/Game/Tut_FirstBlood/Blueprints/HUD_FirstBlood.HUD_FirstBlood_C|SetBlueMode _ashud_first_blood false)
  (Variables|/Game/Tut_FirstBlood/Blueprints/HUD_FirstBlood.HUD_FirstBlood_C|SetRedMode _ashud_first_blood true))

(event Custom|Green
  (bind _ashud_first_blood (Utilities|Casting|CastToHUD_FirstBlood (HUD|GetHUD (Game|GetPlayerController 0))))
  (Variables|/Game/Tut_FirstBlood/Blueprints/HUD_FirstBlood.HUD_FirstBlood_C|SetBlueMode _ashud_first_blood false)
  (Variables|/Game/Tut_FirstBlood/Blueprints/HUD_FirstBlood.HUD_FirstBlood_C|SetRedMode _ashud_first_blood false)
  (Variables|/Game/Tut_FirstBlood/Blueprints/HUD_FirstBlood.HUD_FirstBlood_C|SetGreenMode _ashud_first_blood true))

(event Custom|Blue
  (bind _ashud_first_blood (Utilities|Casting|CastToHUD_FirstBlood (HUD|GetHUD (Game|GetPlayerController 0))))
  (Variables|/Game/Tut_FirstBlood/Blueprints/HUD_FirstBlood.HUD_FirstBlood_C|SetRedMode _ashud_first_blood false)
  (Variables|/Game/Tut_FirstBlood/Blueprints/HUD_FirstBlood.HUD_FirstBlood_C|SetGreenMode _ashud_first_blood false)
  (Variables|/Game/Tut_FirstBlood/Blueprints/HUD_FirstBlood.HUD_FirstBlood_C|SetBlueMode _ashud_first_blood true))

(event EventBeginPlay
  (CallFunction|Blue)
  (Rendering|Material|SetVectorParameterValue (Variables|Default|GetcharacterMat) "BodyColor" "(R=0.013376,G=0.000000,B=1.000000,A=1.000000)" :!class /Script/Engine.MaterialInstanceDynamic))

(event Collision|EventActorBeginOverlap
  (params (OtherActor :type Actor%20Object%20Reference)))

(event EventTick
  (params (DeltaSeconds :type Float%20%28single-precision%29)))

(event Input|KeyboardEvents|1
  (params (Key :type Key%20Structure :default "None"))
  (:Pressed
    (CallFunction|Red)
    (Rendering|Material|SetVectorParameterValue (Variables|Default|GetcharacterMat) "BodyColor" "(R=1.000000,G=0.000000,B=0.000000,A=1.000000)" :!class /Script/Engine.MaterialInstanceDynamic)))

(event Input|KeyboardEvents|2
  (params (Key :type Key%20Structure :default "None"))
  (:Pressed
    (CallFunction|Green)
    (Rendering|Material|SetVectorParameterValue (Variables|Default|GetcharacterMat) "BodyColor" "(R=0.013145,G=1.000000,B=0.000000,A=1.000000)" :!class /Script/Engine.MaterialInstanceDynamic)))

(event Input|KeyboardEvents|3
  (params (Key :type Key%20Structure :default "None"))
  (:Pressed
    (CallFunction|Blue)
    (Rendering|Material|SetVectorParameterValue (Variables|Default|GetcharacterMat) "BodyColor" "(R=0.013376,G=0.000000,B=1.000000,A=1.000000)" :!class /Script/Engine.MaterialInstanceDynamic)))

(fn ConstructionScript
  (bind _returnvalue (Rendering|Material|CreateDynamicMaterialInstance (Variables|Character|GetMesh) 0 0 "None" :!class /Script/Engine.PrimitiveComponent))
  (Variables|Default|SetcharacterMat _returnvalue))